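; BP_PickupItem is a world pickup that adds its item to the interactor's inventory.
; Construction sets the mesh from the item definition's world representation fragment.
; Interact passes the item info to the interactor's InventoryManagerComponent and destroys the actor, doing nothing if that component is missing.
; Interaction getters supply type, hold duration, tap count, a prompt with name and count, and a point above the mesh.
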(event `/Game/_InteractSystem/Interfaces/BPI_Interactable.Interact`
  (params (Interactor :type "Actor Object Reference"))
  (bind _returnvalue (`self.GetComponentByClass` Interactor "/Game/_InventorySystem/Manager/InventoryManagerComponent.InventoryManagerComponent_C"))
  (`/Engine/EditorBlueprintResources/StandardMacros.IsValid` _returnvalue
    (:`Is Valid`
      (`/Game/_InventorySystem/Manager/InventoryManagerComponent.AddItem` _returnvalue (`self.InventoryItemInfo`))
      (`self.K2_DestroyActor`))))

(event `self.ReceiveActorBeginOverlap`
  (params (OtherActor :type "Actor Object Reference")))

(fn `GetHoldDuration`
  (returns (Duration :type "Float (double-precision)"))
  (return (`self.HoldDuration`)))

(fn `GetInteractionType`
  (returns (InteractionType :type "/Game/_InteractSystem/Data/E_Interactiontype Enum"))
  (return (`self.InteractionType`)))

(fn `GetInteractLocation`
  (returns (Location :type "Vector Structure"))
  (return (+ (`SceneComponent.K2_GetComponentLocation` (`self.ItemMesh`)) (0.0 0.0 40.0))))

(fn `GetInteractMessage`
  (returns (Message :type Text))
  (bind (_inventoryiteminfo_itemdefinition _inventoryiteminfo_count) (break `/Game/_InventorySystem/Types/S_InventoryItemInfo` (`self.InventoryItemInfo`)))
  (return (`|FormatText` "to Pickup {ItemName} x {Count}" (defaults `Object` _inventoryiteminfo_itemdefinition) _inventoryiteminfo_count)))

(fn `GetTapCount`
  (returns (TapCount :type Integer))
  (return (`self.TapCount`)))

(fn `UserConstructionScript`
  (bind _inventoryiteminfo_itemdefinition (break `/Game/_InventorySystem/Types/S_InventoryItemInfo` (`self.InventoryItemInfo`)))
  (bind _returnvalue (`ItemDefinition.FindFragmentByClass` _inventoryiteminfo_itemdefinition "/Script/Ali_InventorySystem.ItemWorldRepresentationFragment"))
  (`/Engine/EditorBlueprintResources/StandardMacros.IsValid` _returnvalue
    (:`Is Valid`
      (`StaticMeshComponent.SetStaticMesh` (`self.ItemMesh`) (`ItemWorldRepresentationFragment.ItemMesh` _returnvalue)))))