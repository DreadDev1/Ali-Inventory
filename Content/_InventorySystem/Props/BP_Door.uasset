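; BP_Door is an interactable locked door that opens by sliding its panel down when the interactor carries a usable lockpick.
; Interact searches the interactor's inventory manager, spends one use of the first lockpick with uses left via BP_LimitedUseFragment, and blocks further interaction.
; OpenDoor plays a sound and runs a timeline that lerps the panel's height.
; Blocked doors, missing inventories or missing lockpicks play an invalid-action sound.
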(event `self.ReceiveBeginPlay`
  (bind (_returnvalue_x _returnvalue_y _returnvalue_z) (`KismetMathLibrary.BreakVector` (`SceneComponent.K2_GetComponentLocation` (`self.DoorPanel`))))
  (bind _output_get (set `self.CloseZLocation` _returnvalue_z))
  (set `self.OpenZLocation` (- _output_get 230.0)))

(event `OpenDoor`
  (bind _doorpanel (`self.DoorPanel`))
  (bind (_returnvalue_x _returnvalue_y) (`KismetMathLibrary.BreakVector` (`SceneComponent.K2_GetComponentLocation` _doorpanel)))
  (`GameplayStatics.PlaySoundAtLocation` null (`self.K2_GetActorLocation`) (struct) 1.0 1.0 0.0 null null null null)
  (bind (_direction _zlocation) (`Timeline|Timeline`)
    (:`Update`
      (`SceneComponent.K2_SetWorldLocation` _doorpanel (`KismetMathLibrary.MakeVector` _returnvalue_x _returnvalue_y (`KismetMathLibrary.Lerp` (`self.CloseZLocation`) (`self.OpenZLocation`) _zlocation)) false false))))

(event `/Game/_InteractSystem/Interfaces/BPI_Interactable.Interact`
  (params (Interactor :type "Actor Object Reference"))
  (bind _returnvalue (`self.GetComponentByClass` Interactor "/Game/_InventorySystem/Manager/InventoryManagerComponent.InventoryManagerComponent_C"))
  (`KismetSystemLibrary.PrintString` "Hello")
  (`self.InteractionBlocked`
    (:`then`
      (`GameplayStatics.PlaySoundAtLocation` "/Engine/VREditor/Sounds/UI/Invalid_Action.Invalid_Action" (`self.K2_GetActorLocation`) (struct) 1.0 1.0 0.0 null null null null :!label _label))
    (:`else`
      (`/Engine/EditorBlueprintResources/StandardMacros.IsValid` _returnvalue
        (:`Is Valid`
          (bind _inventoryitems (`/Game/_InventorySystem/Manager/InventoryManagerComponent.FindAllItems` _returnvalue "/Game/_InventorySystem/Items/Item_Lockpick.Item_Lockpick_C"))
          (if (`KismetArrayLibrary.Array_IsNotEmpty` _inventoryitems)
            (for _array_element _inventoryitems
              (bind _returnvalue_2 (`ItemInstance.FindFragmentByClass` (break `/Game/_InventorySystem/Types/S_InventoryItem` _array_element) "/Game/_InventorySystem/Fragments/BP_LimitedUseFragment.BP_LimitedUseFragment_C"))
              (if (`/Game/_InventorySystem/Fragments/BP_LimitedUseFragment.HasUsesLeft` _returnvalue_2 (break `/Game/_InventorySystem/Types/S_InventoryItem` _array_element))
                (`self.OpenDoor`)
                (set `self.InteractionBlocked` true)
                (`/Game/_InventorySystem/Fragments/BP_LimitedUseFragment.DecrementUsesLeft` _returnvalue_2 (break `/Game/_InventorySystem/Types/S_InventoryItem` _array_element))
                (break)))
            (else
              (goto _label))))
        (:`Is Not Valid`
          (goto _label))))))

(fn `GetHoldDuration`
  (returns (Duration :type "Float (double-precision)"))
  (return 0.0))

(fn `GetInteractionType`
  (returns (InteractionType :type "/Game/_InteractSystem/Data/E_Interactiontype Enum"))
  (return "NewEnumerator1"))

(fn `GetInteractLocation`
  (returns (Location :type "Vector Structure"))
  (return (0.0 0.0 0.0)))

(fn `GetInteractMessage`
  (returns (Message :type Text))
  (return ""))

(fn `GetTapCount`
  (returns (TapCount :type Integer))
  (return 0))

(fn `UserConstructionScript`)