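; BP_PickupItem is an interactable world pickup that hands its InventoryItemInfo to the interactor's InventoryManagerComponent, then destroys itself.
; The construction script sets the static mesh from the item definition's WorldRepresentation fragment, so one actor displays any item.
; Interaction interface functions supply a prompt with item name and count, a location above the mesh, and the interaction type, hold duration and tap count.
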(event `/Game/_InteractionSystem/BPI_Interactable.Interact`
  (params (Interactor :type "Actor Object Reference"))
  (bind _returnvalue (`self.GetComponentByClass` Interactor "/Game/_InventorySystem/InventoryManagerComponent.InventoryManagerComponent_C"))
  (`/Engine/EditorBlueprintResources/StandardMacros.IsValid` _returnvalue
    (:`Is Valid`
      (`/Game/_InventorySystem/InventoryManagerComponent.AddItem` _returnvalue (`self.InventoryItemInfo`))
      (`self.K2_DestroyActor`))))

(fn `GetHoldDuration`
  (returns (duration :type "Float (double-precision)"))
  (return 0.5))

(fn `GetInteractionLocation`
  (returns (Location :type "Vector Structure"))
  (return (+ (`SceneComponent.K2_GetComponentLocation` (`self.StaticMesh`)) (0.0 0.0 40.0))))

(fn `GetInteractionPrompt`
  (returns (Value :type Text))
  (bind (_inventoryiteminfo_itemdefinition _inventoryiteminfo_count) (break `/Game/_InventorySystem/Types/S_InventoryItemInfo` (`self.InventoryItemInfo`)))
  (return (`|FormatText` "To Pickup {ItemName} x{Count}" (defaults `Object` _inventoryiteminfo_itemdefinition) _inventoryiteminfo_count)))

(fn `GetInteractionType`
  (returns (Type :type "/Game/_InteractionSystem/E_InteractionType Enum"))
  (return "NewEnumerator0"))

(fn `GetTapCount`
  (returns (Value :type Integer))
  (return 3))

(fn `UserConstructionScript`
  (bind _inventoryiteminfo_itemdefinition (break `/Game/_InventorySystem/Types/S_InventoryItemInfo` (`self.InventoryItemInfo`)))
  (bind _returnvalue (`ItemDefinition.FindFragmentByClass` _inventoryiteminfo_itemdefinition "/Script/InventorySystem.InventoryItemFragment_WorldRepresentation"))
  (`/Engine/EditorBlueprintResources/StandardMacros.IsValid` _returnvalue
    (:`Is Valid`
      (`StaticMeshComponent.SetStaticMesh` (`self.StaticMesh`) (`InventoryItemFragment_WorldRepresentation.ItemMesh` _returnvalue)))))