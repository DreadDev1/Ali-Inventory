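; BP_ItemFragment_LimitedUse is an inventory item fragment that gives items a limited number of uses.
; On instance creation it seeds the Item.Stat.UsesLeft stat tag from MaxNumberOfUses, so the count lives on each item instance rather than the fragment.
; Helper functions decrement that stat, clamped so it never drops below zero, and report whether any uses remain.
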(event `self.OnInstanceCreated`
  (params (ItemInstance :type "ItemInstance Object Reference"))
  (`ItemInstance.SetStatValue` ItemInstance (struct :`TagName` "Item.Stat.UsesLeft") (`KismetMathLibrary.Conv_IntToDouble` (`self.MaxNumberOfUses`))))

(fn `DecrementUsesLeft`
  (params (ItemInstance :type "ItemInstance Object Reference"))
  (`ItemInstance.SetStatValue` ItemInstance (struct :`TagName` "Item.Stat.UsesLeft") (`KismetMathLibrary.FClamp` (- (`ItemInstance.GetStatValue` ItemInstance (struct :`TagName` "Item.Stat.UsesLeft")) 1.0) 0.0 99999.0)))

(fn `HasUsesLeft`
  (params (ItemInstance :type "ItemInstance Object Reference"))
  (returns (ReturnValue :type Boolean))
  (return (> (`ItemInstance.GetStatValue` ItemInstance (struct :`TagName` "Item.Stat.UsesLeft")) 0.0)))