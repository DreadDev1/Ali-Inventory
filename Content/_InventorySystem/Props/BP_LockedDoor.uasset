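; BP_LockedDoor is an interactable door that a player opens by picking its lock with a lockpick from their inventory.
; Interact searches the interactor's InventoryManagerComponent for lockpicks, spends a use from the first with uses left via its LimitedUse item fragment, then blocks further interaction.
; A timeline lowers the door panel with a sound.
; Blocked attempts or missing lockpicks play an invalid-action sound.
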(event `self.ReceiveBeginPlay`
  (bind (_returnvalue_x _returnvalue_y _returnvalue_z) (`KismetMathLibrary.BreakVector` (`SceneComponent.K2_GetComponentLocation` (`self.DoorPanel`))))
  (bind _output_get (set `self.CloseZLocation` _returnvalue_z))
  (set `self.OpenZLocation` (- _output_get 230.0)))

(event `OpenDoor`
  (bind _doorpanel (`self.DoorPanel`))
  (bind (_returnvalue_x _returnvalue_y) (`KismetMathLibrary.BreakVector` (`SceneComponent.K2_GetComponentLocation` _doorpanel)))
  (`GameplayStatics.PlaySoundAtLocation` "/Engine/VREditor/Sounds/UI/Enter_Play.Enter_Play" (`self.K2_GetActorLocation`) (struct) 1.0 1.0 0.0 null null null null)
  (bind (_direction _zlocationalpha) (`Timeline|OpenDoorTimeline`)
    (:`Update`
      (`SceneComponent.K2_SetWorldLocation` _doorpanel (`KismetMathLibrary.MakeVector` _returnvalue_x _returnvalue_y (`KismetMathLibrary.Lerp` (`self.CloseZLocation`) (`self.OpenZLocation`) _zlocationalpha)) false false))))

(event `/Game/_InteractionSystem/BPI_Interactable.Interact`
  (params (Interactor :type "Actor Object Reference"))
  (bind _returnvalue (`self.GetComponentByClass` Interactor "/Game/_InventorySystem/InventoryManagerComponent.InventoryManagerComponent_C"))
  (`self.InteractionBlocked`
    (:`then`
      (`GameplayStatics.PlaySoundAtLocation` "/Engine/VREditor/Sounds/UI/Invalid_Action.Invalid_Action" (`self.K2_GetActorLocation`) (struct) 1.0 1.0 0.0 null null null null :!label _label))
    (:`else`
      (`/Engine/EditorBlueprintResources/StandardMacros.IsValid` _returnvalue
        (:`Is Valid`
          (bind _items (`/Game/_InventorySystem/InventoryManagerComponent.FindAllItems` _returnvalue "/Game/_InventorySystem/Items/Item_LockPick.Item_LockPick_C"))
          (if (`KismetArrayLibrary.Array_IsNotEmpty` _items)
            (for _array_element _items
              (bind _returnvalue_2 (`ItemInstance.FindFragmentByClass` (break `/Game/_InventorySystem/Types/S_InventoryItem` _array_element) "/Game/_InventorySystem/Fragments/BP_ItemFragment_LimitedUse.BP_ItemFragment_LimitedUse_C"))
              (if (`/Game/_InventorySystem/Fragments/BP_ItemFragment_LimitedUse.HasUsesLeft` _returnvalue_2 (break `/Game/_InventorySystem/Types/S_InventoryItem` _array_element))
                (`self.OpenDoor`)
                (set `self.InteractionBlocked` true)
                (`/Game/_InventorySystem/Fragments/BP_ItemFragment_LimitedUse.DecrementUsesLeft` _returnvalue_2 (break `/Game/_InventorySystem/Types/S_InventoryItem` _array_element))
                (break)))
            (else
              (goto _label))))
        (:`Is Not Valid`
          (goto _label))))))

(fn `GetHoldDuration`
  (returns (duration :type "Float (double-precision)"))
  (return 0.0))

(fn `GetInteractionLocation`
  (returns (Location :type "Vector Structure"))
  (return (0.0 0.0 0.0)))

(fn `GetInteractionPrompt`
  (returns (Value :type Text))
  (return "to Pick The Lock"))

(fn `GetInteractionType`
  (returns (Type :type "/Game/_InteractionSystem/E_InteractionType Enum"))
  (return "NewEnumerator0"))

(fn `GetTapCount`
  (returns (Value :type Integer))
  (return 0))

(fn `UserConstructionScript`)